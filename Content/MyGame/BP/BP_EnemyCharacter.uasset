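; Enemy character Blueprint that chases the player on sight and plays a mudra-pose montage as its attack on arrival.
; PawnSensing sets IsSeeingPlayer, which is never cleared here, and calls FollowPlayer to run AIMoveTo toward player character 0.
; On move success, CanAttack gates the montage and returns after a delay of its length, though each FollowPlayer call also re-enables it.
; No damage logic is present.
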(event OnSeePawn(PawnSensing)
  (params (Pawn :type Pawn%20Object%20Reference))
  (Variables|Default|SetIsSeeingPlayer true)
  (CallFunction|FollowPlayer))

(event Custom|FollowPlayer
  (Variables|Default|SetCanAttack true)
  (if (Variables|Default|GetIsSeeingPlayer)
    (AI|AIMoveTo self "0, 0, 0" (Game|GetPlayerCharacter 0) 5.0 false
      (:OnSuccess
        (if (Variables|Default|GetCanAttack)
          (Variables|Default|SetCanAttack false)
          (bind _returnvalue (Animation|PlayAnimMontage "/Game/MudraSamples/Animations/MudraSamples/MANNY/AS_Anime_Mudra_Pose_01_Ox_Manny_Montage.AS_Anime_Mudra_Pose_01_Ox_Manny_Montage" 1.0 "None"))
          (Utilities|FlowControl|Delay _returnvalue)
          (Variables|Default|SetCanAttack true))))))

(event EventBeginPlay)

(event Collision|EventActorBeginOverlap
  (params (OtherActor :type Actor%20Object%20Reference)))

(event EventTick
  (params (DeltaSeconds :type Float%20%28single-precision%29)))

(fn ConstructionScript)